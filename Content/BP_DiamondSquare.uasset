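; Procedural terrain actor that builds a grid mesh with random heights at BeginPlay; despite its name, it runs no diamond-square algorithm.
; CreateVertices fills an X/Y grid with scaled positions, an independent random Z between ZMin and ZMax, and scaled UVs.
; CreateTriangles indexes that grid two triangles per quad.
; The arrays feed one ProceduralMesh section with collision and an assigned material, without computed normals or tangents.
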(event `self.ReceiveBeginPlay`
  (`self.CreateVertices`)
  (`self.CreateTriangles`)
  (`ProceduralMeshComponent.CreateMeshSection_LinearColor` :`self` (`self.ProceduralMesh`) :`Vertices` (`self.Vertices`) :`Triangles` (`self.Triangles`) :`UV0` (`self.UV0`) :`bCreateCollision` true)
  (`PrimitiveComponent.SetMaterial` (`self.ProceduralMesh`) 0 (`self.Material`)))

(fn `CreateTriangles`
  (locals (Vertex :type Integer))
  (for _ (range (`self.XSize`))
    (`KismetArrayLibrary.Array_Add` (`self.Triangles`) (`local.Vertex`))
    (`KismetArrayLibrary.Array_Add` (`self.Triangles`) (+ (`local.Vertex`) 1))
    (`KismetArrayLibrary.Array_Add` (`self.Triangles`) (+ (`self.YSize`) (`local.Vertex`) 1))
    (`KismetArrayLibrary.Array_Add` (`self.Triangles`) (+ (`local.Vertex`) 1))
    (`KismetArrayLibrary.Array_Add` (`self.Triangles`) (+ (`self.YSize`) (`local.Vertex`) 2))
    (`KismetArrayLibrary.Array_Add` (`self.Triangles`) (+ (`self.YSize`) (`local.Vertex`) 1))
    (`/Engine/EditorBlueprintResources/StandardMacros.IncrementInt` (`local.Vertex`)
      (:`  `
        (for _ (range (`self.YSize`))
          (`KismetArrayLibrary.Array_Add` (`self.Triangles`) (`local.Vertex`))
          (`KismetArrayLibrary.Array_Add` (`self.Triangles`) (+ (`local.Vertex`) 1))
          (`KismetArrayLibrary.Array_Add` (`self.Triangles`) (+ (`self.YSize`) (`local.Vertex`) 1))
          (`KismetArrayLibrary.Array_Add` (`self.Triangles`) (+ (`local.Vertex`) 1))
          (`KismetArrayLibrary.Array_Add` (`self.Triangles`) (+ (`self.YSize`) (`local.Vertex`) 2))
          (`KismetArrayLibrary.Array_Add` (`self.Triangles`) (+ (`self.YSize`) (`local.Vertex`) 1))
          (`/Engine/EditorBlueprintResources/StandardMacros.IncrementInt` (`local.Vertex`))))))
  (`/Engine/EditorBlueprintResources/StandardMacros.IncrementInt` (`local.Vertex`)))

(fn `CreateVertices`
  (locals (X :type Integer) (Y :type Integer))
  (for _index (range (+ (`self.XSize`) 1))
    (set `local.X` _index)
    (for _index_2 (range (+ (`self.YSize`) 1))
      (set `local.Y` _index_2)
      (`KismetArrayLibrary.Array_Add` (`self.Vertices`) (`KismetMathLibrary.MakeVector` (* (`local.X`) (`self.Scale`)) (* (`local.Y`) (`self.Scale`)) (`KismetMathLibrary.RandomFloatInRange` (`self.ZMin`) (`self.ZMax`))))
      (`KismetArrayLibrary.Array_Add` (`self.UV0`) (`KismetMathLibrary.MakeVector2D` (* (`local.X`) (`self.UVScale`)) (* (`local.Y`) (`self.UVScale`)))))))

(fn `UserConstructionScript`)